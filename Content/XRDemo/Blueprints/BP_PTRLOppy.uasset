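; Oppy character Blueprint with a flickering flame and point light, plus jump start and stop events.
; Every tick, Perlin noise drives both the light intensity and the flame material's NoiseFactor.
; The light trails a bobbing flame pivot with interpolation, and the flame tilts by that lag, blending from the capsule's rotation.
; Jump events set flags on Oppi_ABP when grounded, while stopping mid-fall calls StopJumping.
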(event `self.ReceiveBeginPlay`
  (bind _returnvalue (`PrimitiveComponent.CreateDynamicMaterialInstance` (`self.Mesh`) 0 null "None"))
  (set `self.DynMat` _returnvalue)
  (bind _returnvalue_2 (`PrimitiveComponent.CreateDynamicMaterialInstance` (`self.Flame`) 0 null "None"))
  (set `self.FlameDynMat` _returnvalue_2))

(event `self.ReceiveTick`
  (params (DeltaSeconds :type "Float (single-precision)"))
  (`self.Update Light`))

(event `InitiateJump`
  ;[1 1 1] Jump events
  (if (`NavMovementComponent.IsMovingOnGround` (`self.CharacterMovement`))
    (bind _asoppi_abp (cast `/Game/XRDemo/Characters/Oppy/Animations/Oppi_ABP` (`SkeletalMeshComponent.GetAnimInstance` (`self.Mesh`))))
    (set `/Game/XRDemo/Characters/Oppy/Animations/Oppi_ABP.Jump` true _asoppi_abp)))

(event `StopJump`
  ;[1 1 1] Jump events
  (if (`NavMovementComponent.IsFalling` (`self.CharacterMovement`))
    (`self.StopJumping`)
    (else
      (bind _asoppi_abp (cast `/Game/XRDemo/Characters/Oppy/Animations/Oppi_ABP` (`SkeletalMeshComponent.GetAnimInstance` (`self.Mesh`))))
      (if (`/Game/XRDemo/Characters/Oppy/Animations/Oppi_ABP.Jump` _asoppi_abp)
        (set `/Game/XRDemo/Characters/Oppy/Animations/Oppi_ABP.BreakJump` true _asoppi_abp)))))

(fn `Update Light`
  (locals (CurrentValue :type "Float (single-precision)" :default 0.0))
  (bind _flame (`self.Flame`))
  (bind _returnvalue (- (`SceneComponent.K2_GetComponentLocation` (`self.PointLight`)) (`SceneComponent.K2_GetComponentLocation` (`self.FlamePivot`))))
  (`|ExecutionSequence`
    (:`then_0`
      (set `local.CurrentValue` (`KismetMathLibrary.Abs` (`KismetMathLibrary.PerlinNoise1D` (* (`GameplayStatics.GetTimeSeconds`) 2.0))))
      (`LightComponent.SetIntensity` (`self.PointLight`) (`KismetMathLibrary.Lerp` (`self.LightPulseMaxIntensity`) 2.0 (`local.CurrentValue`)))
      (`MaterialInstanceDynamic.SetScalarParameterValue` (`self.FlameDynMat`) "NoiseFactor" (`local.CurrentValue`)))
    (:`then_1`
      (`SceneComponent.K2_SetWorldLocation` (`self.PointLight`) (`KismetMathLibrary.VInterpTo` (`SceneComponent.K2_GetComponentLocation` (`self.PointLight`)) (+ (`SceneComponent.K2_GetComponentLocation` (`self.FlamePivot`)) (* (`KismetMathLibrary.Vector_Up`) (* (`KismetMathLibrary.Sin` (* (`GameplayStatics.GetTimeSeconds`) 2.0)) 1.0))) (`GameplayStatics.GetWorldDeltaSeconds`) 10.0) false false)
      (`SceneComponent.K2_SetWorldRotation` _flame (`KismetMathLibrary.RInterpTo` (`SceneComponent.K2_GetComponentRotation` _flame) (`KismetMathLibrary.RLerp` (`SceneComponent.K2_GetComponentRotation` (`self.CapsuleComponent`)) (`KismetMathLibrary.MakeRotFromZX` _returnvalue (`KismetMathLibrary.Vector_Up`)) (`KismetMathLibrary.MapRangeClamped` (`KismetMathLibrary.VSize` _returnvalue) 1.0 20.0 0.0 1.0) true) (`GameplayStatics.GetWorldDeltaSeconds`) 10.0) false false))))

(fn `UserConstructionScript`)